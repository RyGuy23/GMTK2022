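; Parent enemy projectile Blueprint that damages the first-person player and destroys itself on overlap or at maximum range.
; BeginPlay records the hand_R socket of the first EnemyBp found as the origin, and Tick compares distance from it against ProjectileRange.
; Any mesh overlap applies DamageAmount once to the FirstPersonCharacter, without checking what was hit.
; An attach-to-hand_R fragment is left unconnected.
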(event `self.ReceiveBeginPlay`
  (bind _returnvalue (`GameplayStatics.GetActorOfClass` "/Game/Blueprints/EnemyBp.EnemyBp_C"))
  (set `self.StartLocation` (`SceneComponent.GetSocketLocation` (`/Game/Blueprints/EnemyBp.SkeletalMesh` _returnvalue) "hand_R")))

(event `self.ReceiveTick`
  (params (DeltaSeconds :type "Float (single-precision)"))
  (if (>= (`KismetMathLibrary.VSize` (- (`self.StartLocation`) (`self.K2_GetActorLocation`))) (`self.ProjectileRange`))
    (`/Engine/EditorBlueprintResources/StandardMacros.DoOnce` false
      (:`Completed`
        (`self.K2_DestroyActor`)))))

(event `self.ProjectileMesh.OnComponentBeginOverlap`
  (params (OverlappedComponent :type "PrimitiveComponent Object Reference") (OtherActor :type "Actor Object Reference") (OtherComp :type "PrimitiveComponent Object Reference") (OtherBodyIndex :type Integer) (bFromSweep :type Boolean) (SweepResult :type "HitResult Structure (by ref)"))
  (bind _returnvalue (`GameplayStatics.GetActorOfClass` "/Game/FirstPersonBP/Blueprints/FirstPersonCharacter.FirstPersonCharacter_C"))
  (`/Engine/EditorBlueprintResources/StandardMacros.DoOnce` false
    (:`Completed`
      (`GameplayStatics.ApplyDamage` _returnvalue (`KismetMathLibrary.Conv_IntToDouble` (`self.DamageAmount`)) null self)
      (`self.K2_DestroyActor`))))

(fn `UserConstructionScript`)