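; Rook enemy that shoots projectiles at the first-person player when in detection range and resets its aim otherwise.
; Tick runs the range check every frame, while a Delay throttles firing to about once per second.
; Shots turn the actor toward the player and lead the target by velocity scaled with distance.
; Damage plays hit feedback; death drops a random power-up die, spawns effects and increments the player's kill count.
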(event `self.ReceiveBeginPlay`
  (`|ExecutionSequence`
    (:`then_0`
      (bind _asfirst_person_character (cast `/Game/FirstPersonBP/Blueprints/FirstPersonCharacter` (`GameplayStatics.GetPlayerCharacter` 0)))
      (set `self.PlayerRef` _asfirst_person_character))
    (:`then_1`
      (bind _outactors (`GameplayStatics.GetAllActorsOfClass` "/Game/FirstPersonBP/Blueprints/FirstPersonCharacter.FirstPersonCharacter_C"))
      (set `self.Target` (`|GetArrayItem` _outactors)))))

(event `self.ReceiveTick`
  (params (DeltaSeconds :type "Float (single-precision)"))
  (`|ExecutionSequence`
    (:`then_0`
      ;[1 1 1] Change this for bullet speed
      (`KismetSystemLibrary.Delay` 1.0)
      (if (`self.InRange?`)
        (`self.SpawnProjectile`)
        (else
          (`self.StopFiring`))))
    (:`then_1`
      (`self.RangeCheck`
        (:`then`
          (`self.AimAtTarget`))
        (:`else`
          (`self.ResetAim`))))))

(event `AimAtTarget`
  (`SceneComponent.K2_SetRelativeRotation` (`self.SkeletalMesh`) (`self.AimingLogic`) false false))

(event `ResetAim`
  (`SceneComponent.K2_SetRelativeRotation` (`self.SkeletalMesh`) (`KismetMathLibrary.MakeRotator` 0.0 0.0 -90.0) false false))

(event `self.ReceiveAnyDamage`
  (params (Damage :type "Float (single-precision)") (DamageType :type "DamageType Object Reference") (InstigatedBy :type "Controller Object Reference") (DamageCauser :type "Actor Object Reference"))
  (`GameplayStatics.PlaySound2D` "/Game/Music/sfx_exp_shortest_soft1.sfx_exp_shortest_soft1" 0.7 1.0 0.0 null null)
  (`self.TakingDamage` Damage))

(event `SpawnDice`
  (`self.SpawnDiceMacro`))

(event `StopFiring`
  (set `self.CanShoot` false))

(fn `SpawnProjectile`
  (bind _playerref (`self.PlayerRef`))
  (bind _returnvalue (`SceneComponent.K2_GetComponentLocation` (`self.FiringPoint`)))
  (bind _returnvalue_2 (`SceneComponent.K2_GetComponentLocation` (`Character.Mesh` _playerref)))
  (`/Engine/EditorBlueprintResources/StandardMacros.IsValid` (`self.Target`)
    (:`Is Valid`
      (`self.K2_SetActorRotation` (`KismetMathLibrary.FindLookAtRotation` _returnvalue _returnvalue_2))
      (`|SpawnActorFromClass` "/Game/Blueprints/EnemyRevamp/PawnProjectile2.PawnProjectile2_C" (`KismetMathLibrary.MakeTransform` _returnvalue (`KismetMathLibrary.FindLookAtRotation` _returnvalue (+ _returnvalue_2 (* (`self.GetVelocity` _playerref) (/ (`self.GetDistanceTo` _playerref) 5000.0))))) "Undefined" "OverrideRootScale" null null))
    (:`Is Not Valid`
      (`self.StopFiring`))))

(fn `UserConstructionScript`)