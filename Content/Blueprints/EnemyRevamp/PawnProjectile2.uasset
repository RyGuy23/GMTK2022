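; PawnProjectile2 is an enemy projectile Blueprint that punishes the first-person player on overlap.
; Its collision component casts the overlapping actor to FirstPersonCharacter and checks HasShield.
; A shielded player loses the shield with a debug print, while an unshielded one has movement and input disabled, then the current level reloads after a short delay.
; The file contains no movement or self-destroy logic.
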(event `self.ReceiveTick`
  (params (DeltaSeconds :type "Float (single-precision)")))

(event `self.PawnProjectileCollision.OnComponentBeginOverlap`
  (params (OverlappedComponent :type "PrimitiveComponent Object Reference") (OtherActor :type "Actor Object Reference") (OtherComp :type "PrimitiveComponent Object Reference") (OtherBodyIndex :type Integer) (bFromSweep :type Boolean) (SweepResult :type "HitResult Structure (by ref)"))
  (bind _asfirst_person_character (cast `/Game/FirstPersonBP/Blueprints/FirstPersonCharacter` OtherActor))
  (if (`/Game/FirstPersonBP/Blueprints/FirstPersonCharacter.HasShield` _asfirst_person_character)
    (set `/Game/FirstPersonBP/Blueprints/FirstPersonCharacter.HasShield` false _asfirst_person_character)
    (`KismetSystemLibrary.PrintString` "LostShield")
    (else
      (`CharacterMovementComponent.DisableMovement` (`Character.CharacterMovement` _asfirst_person_character))
      (`self.DisableInput` _asfirst_person_character (`GameplayStatics.GetPlayerController` 0))
      (`KismetSystemLibrary.Delay` 2.0)
      (bind _returnvalue (`GameplayStatics.GetCurrentLevelName` true))
      (`GameplayStatics.OpenLevel` (`KismetStringLibrary.Conv_StringToName` _returnvalue)))))

(fn `UserConstructionScript`)