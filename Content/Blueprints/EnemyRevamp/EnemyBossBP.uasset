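; Chess-themed enemy boss that tracks the first FirstPersonCharacter found in the level and dies when damage depletes its health.
; Each tick RangeCheck stores the target's location and tests detection range, then the mesh rotation is set from AimingLogic, whose interpolation math is left unconnected.
; Death removes the pawn and rook hands, plays an animation, then after a delay destroys the actor before spawning the death effect.
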(event `self.ReceiveAnyDamage`
  (params (Damage :type "Float (single-precision)") (DamageType :type "DamageType Object Reference") (InstigatedBy :type "Controller Object Reference") (DamageCauser :type "Actor Object Reference"))
  (bind _output_get (set `self.Health` (- (`self.Health`) Damage)))
  (if (<= _output_get 0.0)
    (`ActorComponent.K2_DestroyComponent` (`self.PawnHand1`))
    (`ActorComponent.K2_DestroyComponent` (`self.PawnHand2`))
    (`ActorComponent.K2_DestroyComponent` (`self.RookHand1`))
    (`ActorComponent.K2_DestroyComponent` (`self.RookHand2`))
    (`SkeletalMeshComponent.PlayAnimation` (`self.SkeletalMesh`) "/Game/Art/Boss/ChessBoss_Anim_MainRIg_Death.ChessBoss_Anim_MainRIg_Death" false)
    (`KismetSystemLibrary.Delay` 2.0)
    (`self.K2_DestroyActor`)
    (`NiagaraFunctionLibrary.SpawnSystemAttached` "/Game/Art/Effects/PS_Death.PS_Death" (`self.SkeletalMesh`) "None" (0.0 0.0 0.0) (struct) "KeepRelativeOffset")))

(event `AimAtTarget`
  (`SceneComponent.K2_SetRelativeRotation` (`self.SkeletalMesh`) (`self.AimingLogic`) false false))

(event `self.ReceiveTick`
  (params (DeltaSeconds :type "Float (single-precision)"))
  (`self.RangeCheck`)
  (`self.AimAtTarget`))

(event `self.ReceiveBeginPlay`
  (bind _outactors (`GameplayStatics.GetAllActorsOfClass` "/Game/FirstPersonBP/Blueprints/FirstPersonCharacter.FirstPersonCharacter_C"))
  (set `self.Target` (`|GetArrayItem` _outactors)))

(fn `UserConstructionScript`)