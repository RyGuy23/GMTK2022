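; Enemy actor that aims at the first-person player within detection range and shoots projectiles, resetting its aim otherwise.
; Each Tick checks distance and rotates the skeletal mesh toward the target, with a DoOnce gate starting the fire cycle.
; A refire timeline paces projectiles spawned at the hand socket and impulsed toward the player.
; Damage plays a hit animation, and death spawns a random speed or jump dice plus a particle effect.
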(event `self.ReceiveBeginPlay`
  (bind _outactors (`GameplayStatics.GetAllActorsOfClass` "/Game/FirstPersonBP/Blueprints/FirstPersonCharacter.FirstPersonCharacter_C"))
  (set `self.Target` (`|GetArrayItem` _outactors)))

(event `self.ReceiveTick`
  (params (DeltaSeconds :type "Float (single-precision)"))
  (set `self.TargetLocation` (`self.K2_GetActorLocation` (`self.Target`)))
  ;[1 1 1] Checks the targets distance
  (if (<= (`KismetMathLibrary.VSize` (- (`self.K2_GetActorLocation`) (`self.TargetLocation`))) (`self.DetectionRange`))
    (`self.AimAtTarget`)
    (else
      (`self.ResetAim`))))

(event `self.ReceiveAnyDamage`
  (params (Damage :type "Float (single-precision)") (DamageType :type "DamageType Object Reference") (InstigatedBy :type "Controller Object Reference") (DamageCauser :type "Actor Object Reference"))
  (`self.TakingDamage` Damage))

(event `ResetFireTrigger`
  (goto _label :!via `Reset`))

(event `SpawnDice`
  (`self.SpawnDiceMacro`))

(event `AimAtTarget`
  (bind _returnvalue (`KismetMathLibrary.MakeRotator` 0.0 (.pitch (`SceneComponent.RelativeRotation` (`self.SkeletalMesh`))) (.yaw (`SceneComponent.RelativeRotation` (`self.SkeletalMesh`)))))
  (`SceneComponent.K2_SetRelativeRotation` (`self.SkeletalMesh`) (`self.AimingLogic`) false false)
  (if (== _returnvalue _returnvalue :`ErrorTolerance` 1.0)
    (`|ExecutionSequence`
      (:`then_0`
        (`/Engine/EditorBlueprintResources/StandardMacros.DoOnce` false :!label _label
          (:`Completed`
            (set `self.CanShoot` true)
            (`self.StartFiring`)))))
    (else
      (`self.StopFiring`))))

(event `ResetAim`
  (`SceneComponent.K2_SetRelativeRotation` (`self.SkeletalMesh`) (`KismetMathLibrary.MakeRotator` 0.0) false false))

(event `ContinueFiring`
  (if (`self.CanShoot`)
    (if (== (`TimelineComponent.GetPlaybackPosition` (`self.RefireTimeline`)) 0.0) :!label _label_2
      (`self.FireProjectile`)
      (`Timeline|RefireTimeline` :!label _label_3
        (:`Finished`
          (`self.ResetFireTimeline`)
          (`self.ContinueFiring`)
          (`self.StopFiring`))))))

(event `StartFiring`
  (`TimelineComponent.SetTimelineLength` (`self.RefireTimeline`) (`self.RefireDelay`))
  (goto _label_2))

(event `ResetFireTimeline`
  (`|ExecutionSequence`
    (:`then_0`
      (goto _label_3 :!via `Stop`))
    (:`then_1`
      (goto _label_3 :!via `SetNewTime`))))

(event `StopFiring`
  (set `self.CanShoot` false)
  (`self.ResetFireTrigger`))

(event `FireProjectile`
  (`/Engine/EditorBlueprintResources/StandardMacros.IsValid` (`self.Target`)
    (:`Is Valid`
      (bind _returnvalue (`|SpawnActorFromClass` "/Game/Blueprints/OldEnemy/ProjectileParent.ProjectileParent_C" (`KismetMathLibrary.MakeTransform` (.location (`SceneComponent.GetSocketTransform` (`self.SkeletalMesh`) "hand_R" "RTS_World")) (.rotation (`SceneComponent.GetSocketTransform` (`self.SkeletalMesh`) "hand_R" "RTS_World"))) "Undefined" "OverrideRootScale" null null))
      (`PrimitiveComponent.AddImpulse` (`/Game/Blueprints/OldEnemy/ProjectileParent.ProjectileMesh` _returnvalue) (* (`KismetMathLibrary.GetForwardVector` (`KismetMathLibrary.FindLookAtRotation` (`self.K2_GetActorLocation`) (`self.K2_GetActorLocation` (`GameplayStatics.GetPlayerPawn` 0)))) 1500.0) "None" true))
    (:`Is Not Valid`
      (`self.StopFiring`))))

(fn `UserConstructionScript`)