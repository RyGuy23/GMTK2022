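; Parent projectile Blueprint for an enemy attack that damages the first-person player and restarts the level.
; BeginPlay records the hand_R socket of the first EnemyBp found as the start location.
; Any collision overlap sets Hit and increments a counter, without filtering the other actor.
; Tick polls these to apply damage once, print a death message, reload after a delay, and set Dead on repeated hits; its range check triggers nothing.
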(event `self.ReceiveBeginPlay`
  (bind _returnvalue (`GameplayStatics.GetActorOfClass` "/Game/Blueprints/OldEnemy/EnemyBp.EnemyBp_C"))
  (set `self.StartLocation` (`SceneComponent.GetSocketLocation` (`/Game/Blueprints/OldEnemy/EnemyBp.SkeletalMesh` _returnvalue) "hand_R")))

(event `self.ReceiveTick`
  (params (DeltaSeconds :type "Float (single-precision)"))
  (`|ExecutionSequence`
    (:`then_0`
      (if (>= (`KismetMathLibrary.VSize` (- (`self.StartLocation`) (`self.K2_GetActorLocation`))) (`self.ProjectileRange`))
        _))
    (:`then_1`
      (if (`self.Hit?`)
        (bind _returnvalue (`GameplayStatics.GetActorOfClass` "/Game/FirstPersonBP/Blueprints/FirstPersonCharacter.FirstPersonCharacter_C"))
        (`/Engine/EditorBlueprintResources/StandardMacros.DoOnce` false
          (:`Completed`
            (`GameplayStatics.ApplyDamage` _returnvalue (`self.DamageAmount`) null self)
            (`KismetSystemLibrary.PrintString` "you died")
            (`KismetSystemLibrary.Delay` 2.0)
            (bind _returnvalue_2 (`GameplayStatics.GetCurrentLevelName` true))
            (`GameplayStatics.OpenLevel` (`KismetStringLibrary.Conv_StringToName` _returnvalue_2))))))
    (:`then_2`
      (if (>= (`self.HitAmount`) 2.0)
        (set `self.Dead?` true)))))

(event `self.ProjectileCollision.OnComponentBeginOverlap`
  (params (OverlappedComponent :type "PrimitiveComponent Object Reference") (OtherActor :type "Actor Object Reference") (OtherComp :type "PrimitiveComponent Object Reference") (OtherBodyIndex :type Integer) (bFromSweep :type Boolean) (SweepResult :type "HitResult Structure (by ref)"))
  (`GameplayStatics.GetActorOfClass` "/Game/FirstPersonBP/Blueprints/FirstPersonCharacter.FirstPersonCharacter_C")
  (set `self.Hit?` true)
  (bind _output_get (set `self.HitAmount` (+ (`self.HitAmount`) 1.0))))

(fn `UserConstructionScript`)