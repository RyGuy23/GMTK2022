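; Randomizer is a dice Blueprint whose Randomize event prints a random integer from 1 to 6.
; Each Tick, it finds an EnemyPawnBP and copies its EnemyDead state into CanSpawnDice.
; While that flag is true, it spawns another Randomizer at the enemy's DiceSpawnPoint every frame, with no one-shot guard.
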(event `self.ReceiveBeginPlay`)

(event `Randomize`
  (`KismetSystemLibrary.PrintString` (`KismetStringLibrary.Conv_IntToString` (`KismetMathLibrary.RandomIntegerInRange` 1 6))))

(event `self.ReceiveTick`
  (params (DeltaSeconds :type "Float (single-precision)"))
  (`|ExecutionSequence`
    (:`then_0`
      (bind _returnvalue (`GameplayStatics.GetActorOfClass` "/Game/Blueprints/EnemyRevamp/EnemyPawnBP.EnemyPawnBP_C"))
      (if (`/Game/Blueprints/EnemyRevamp/EnemyPawnBP.EnemyDead?` _returnvalue)
        (set `self.CanSpawnDice` true)
        (else
          (set `self.CanSpawnDice` false))))
    (:`then_1`
      (if (`self.CanSpawnDice`)
        (`|SpawnActorFromClass` "Randomizer_C" (`SceneComponent.K2_GetComponentToWorld` (`/Game/Blueprints/EnemyRevamp/EnemyPawnBP.DiceSpawnPoint` _returnvalue)) "Undefined" "OverrideRootScale" null null)))))

(fn `UserConstructionScript`)